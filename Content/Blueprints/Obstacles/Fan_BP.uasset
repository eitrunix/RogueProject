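; Fan obstacle that pushes players and bombs upward while they are inside its Vision volume.
; Overlaps set one shared Floating flag and start looping timer events, which clear themselves once it turns false.
; Players get repeated LaunchCharacter calls, while bombs have their projectile velocity rescaled on Z by direction, with X made positive in local space.
; Enemies trigger the player path, but it stores only the player cast result.
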(event OnComponentBeginOverlap(Vision)
  (params (OverlappedComponent :type Primitive%20Component%20Object%20Reference) (OtherActor :type Actor%20Object%20Reference) (OtherComp :type Primitive%20Component%20Object%20Reference) (OtherBodyIndex :type Integer) (bFromSweep :type Boolean) (SweepResult :type Hit%20Result%20Structure%20%28by%20ref%29))
  (bind _asbomb_bp (Utilities|Casting|CastToBomb_BP OtherActor)
    (:then
      (Variables|MiscVar|Setfloating true)
      (Variables|bombVel|SetTempBomb _asbomb_bp)
      (CallFunction|BombFloating))
    (:CastFailed
      (bind _asmaster_player_bp (Utilities|Casting|CastToMasterPlayer_BP OtherActor)
        (:then
          _)
        (:CastFailed
          (Utilities|Casting|CastToBKUP_MasterEnemy OtherActor)))
      (Variables|MiscVar|Setfloating true)
      (Variables|PlayerVel|SetTempPlayer _asmaster_player_bp)
      (CallFunction|FloatingThing))))

(event OnComponentEndOverlap(Vision)
  (params (OverlappedComponent :type Primitive%20Component%20Object%20Reference) (OtherActor :type Actor%20Object%20Reference) (OtherComp :type Primitive%20Component%20Object%20Reference) (OtherBodyIndex :type Integer))
  (Utilities|Casting|CastToBomb_BP OtherActor
    (:then
      _)
    (:CastFailed
      (Utilities|Casting|CastToMasterPlayer_BP OtherActor
        (:then
          _)
        (:CastFailed
          (Utilities|Casting|CastToBKUP_MasterEnemy OtherActor)))))
  (Variables|MiscVar|Setfloating false))

(event Custom|FloatingThing
  (if (Variables|MiscVar|Getfloating)
    (Utilities|Time|SetTimerbyEvent (delegate Custom|FloatingThing) (Variables|Default|GetPlayerTimeEvent) true)
    (Character|LaunchCharacter (Variables|PlayerVel|GetTempPlayer) (Math|Vector|MakeVector 0.0 0.0 (Variables|PlayerVel|GetUpForce)) true true)
    (else
      (Utilities|Time|SetTimerbyEvent (delegate Custom|FloatingThing) 0.0))))

(event Custom|BombFloating
  (bind _tempbomb (Variables|bombVel|GetTempBomb))
  (bind _returnvalue (Transformation|GetVelocity _tempbomb))
  (if (Variables|MiscVar|Getfloating)
    (Utilities|Time|SetTimerbyEvent (delegate Custom|BombFloating) (Variables|Default|GetBombtimeEvent) true)
    (Variables|Default|SetTempProjMove (Variables|/Game/Blueprints/Projectiles/Bomb_BP.Bomb_BP_C|GetProjectileMovement _tempbomb))
    (Variables|bombVel|SettempXVel (.x _returnvalue))
    (Variables|bombVel|SettempZVel (.z _returnvalue))
    (Variables|bombVel|SettempYVel (.y _returnvalue))
    (if (> (Variables|bombVel|GettempXVel) 0.0)
      (if (> (Variables|bombVel|GettempZVel) 0.0)
        (Game|Components|ProjectileMovement|SetVelocityinLocalSpace (Variables|Default|GetTempProjMove) (Math|Vector|MakeVector (Variables|bombVel|GettempXVel) (Variables|bombVel|GettempYVel) (* (Variables|bombVel|GettempZVel) (Variables|bombVel|GetBombUpForce))))
        (else
          (Game|Components|ProjectileMovement|SetVelocityinLocalSpace (Variables|Default|GetTempProjMove) (Math|Vector|MakeVector (Variables|bombVel|GettempXVel) (Variables|bombVel|GettempYVel) (* (Variables|bombVel|GettempZVel) (- (Variables|bombVel|GetnegForceBOmb) (Variables|bombVel|GetBombUpForce)))))))
      (elif (> (Variables|bombVel|GettempZVel) 0.0)
        (Game|Components|ProjectileMovement|SetVelocityinLocalSpace (Variables|Default|GetTempProjMove) (Math|Vector|MakeVector (* (Variables|bombVel|GettempXVel) -1.0) (Variables|bombVel|GettempYVel) (* (Variables|bombVel|GettempZVel) (Variables|bombVel|GetBombUpForce))))
        (else
          (Game|Components|ProjectileMovement|SetVelocityinLocalSpace (Variables|Default|GetTempProjMove) (Math|Vector|MakeVector (* (Variables|bombVel|GettempXVel) -1.0) (Variables|bombVel|GettempYVel) (* (Variables|bombVel|GettempZVel) (- (Variables|bombVel|GetnegForceBOmb) (Variables|bombVel|GetBombUpForce))))))))
    (else
      (Utilities|Time|SetTimerbyEvent (delegate Custom|BombFloating) 0.0))))

(event EventBeginPlay)

(event Collision|EventActorBeginOverlap
  (params (OtherActor :type Actor%20Object%20Reference)))

(event EventTick
  (params (DeltaSeconds :type Float%20%28single-precision%29)))

(fn ConstructionScript)