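; Trampoline obstacle that springs bombs and players upward when they overlap its collider.
; The overlap stores the actor and runs BounceEvent, which casts in turn to bomb, player and enemy.
; Bombs get an upward local projectile velocity and players get LaunchCharacter; enemies share the player's launch node, which targets only the player cast.
; The flipbook switches to the spring animation, then returns to idle after a short delay.
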(event OnComponentBeginOverlap(Collider)
  (params (OverlappedComponent :type Primitive%20Component%20Object%20Reference) (OtherActor :type Actor%20Object%20Reference) (OtherComp :type Primitive%20Component%20Object%20Reference) (OtherBodyIndex :type Integer) (bFromSweep :type Boolean) (SweepResult :type Hit%20Result%20Structure%20%28by%20ref%29))
  (Variables|Default|SetOther%20Actor OtherActor)
  (CallFunction|BounceEvent))

(event Custom|BounceEvent
  (bind _paperflipbook (Variables|Default|GetPaperFlipbook))
  (bind _other_actor (Variables|Default|GetOther%20Actor))
  (bind _asbomb_bp (Utilities|Casting|CastToBomb_BP _other_actor)
    (:then
      (Game|Components|ProjectileMovement|SetVelocityinLocalSpace (Variables|/Game/Blueprints/Projectiles/Bomb_BP.Bomb_BP_C|GetProjectileMovement _asbomb_bp) "0, 0,500.000000")
      (Sprite|SetFlipbook _paperflipbook "/Game/Art_Textures/Traps/Trampoline/Anims/Jump__28x28__Spring.Jump__28x28__Spring"))
    (:CastFailed
      (bind _asmaster_player_bp (Utilities|Casting|CastToMasterPlayer_BP _other_actor)
        (:then
          _)
        (:CastFailed
          (Utilities|Casting|CastToBKUP_MasterEnemy _other_actor)))
      (Sprite|SetFlipbook _paperflipbook "/Game/Art_Textures/Traps/Trampoline/Anims/Jump__28x28__Spring.Jump__28x28__Spring")
      (Character|LaunchCharacter _asmaster_player_bp "0, 0,500.000000" false true)))
  (Utilities|FlowControl|Delay 0.5)
  (Sprite|SetFlipbook (Variables|Default|GetPaperFlipbook) "/Game/Art_Textures/Traps/Trampoline/Anims/Idle_Spring_Flipbook.Idle_Spring_Flipbook"))

(event EventBeginPlay)

(event Collision|EventActorBeginOverlap
  (params (OtherActor :type Actor%20Object%20Reference)))

(event EventTick
  (params (DeltaSeconds :type Float%20%28single-precision%29)))

(fn ConstructionScript)