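; Dungeon generator actor that builds a room layout on BeginPlay and spawns room Blueprints with a camera each.
; Only the first loop pass creates an area: a rectangular tile grid with random extents from a seeded stream, rerollable through a construction-script toggle.
; Each scaled tile becomes a room; the first is the starting room, whose camera goes to the Game Instance, others follow RandomRoomPick.
; Neighbor-tile testing is unfinished and never runs.
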(event Custom|GenerateMap
  (for _index (range 0 (- (Variables|MapSettings|GetRoomCount) 1))
    (if (== _index 0)
      (bind (_floortiles _root_location _extents) (CallFunction|MakeDungeonArea (Variables|Default|GetPrevLocation)))
      (Variables|Default|SetDungeonMaps _floortiles)
      (Utilities|Map|Add (Variables|RandomRoom|GetRooms) _root_location _extents)))
  (CallFunction|SpawnMaps))

(event EventBeginPlay
  (CallFunction|GenerateMap))

(fn ConstructionScript
  (Utilities|FlowControl|Sequence
    (:then_0
      ;[1 1 1] OnClick NewSeed, Get New Random Seed
      (if (Variables|EditorTools|GetNewSeed)
        (Variables|EditorTools|SetNewSeed false)
        (bind _output_get (Variables|MapSettings|SetSeed (Math|Random|RandomInteger 900000)))
        (Math|Random|SetRandomStreamSeed (Variables|Default|GetStream) _output_get)))
    (:then_1
      ;[1 1 1] Manual Update Stream W Seed
      (Math|Random|SetRandomStreamSeed (Variables|Default|GetStream) (Variables|MapSettings|GetSeed)))))

(fn MakeDungeonArea
  (params (Location :type Int%20Vector%20Structure))
  (bind _roomsize_min (Variables|MapSettings|GetRoomSize_Min))
  (bind _roomsize_max (Variables|MapSettings|GetRoomSize_Max))
  (bind _stream (Variables|Default|GetStream))
  ;[1 1 1] Get Random X and Y extents and make array of tiles from X,Y Added to root position
  (LocalVariables|SetRootLocation Location)
  (LocalVariables|SetOutX (Math|Random|RandomIntegerinRangefromStream _roomsize_min _roomsize_max _stream))
  (LocalVariables|SetOutY (Math|Random|RandomIntegerinRangefromStream _roomsize_min _roomsize_max _stream))
  (for _index (range 0 (- (* (LocalVariables|GetOutX) (LocalVariables|GetOutY)) 1))
    (Utilities|Array|Add (LocalVariables|GetTiles) (Utilities|Struct|MakeIntVector (+ (/ _index (LocalVariables|GetOutY)) (.X (Utilities|Struct|BreakIntVector (LocalVariables|GetRootLocation)))) (.Z (Utilities|Struct|BreakIntVector (LocalVariables|GetRootLocation))) (+ (Math|Integer|%(Integer) _index (LocalVariables|GetOutY)) (.Y (Utilities|Struct|BreakIntVector (LocalVariables|GetRootLocation)))))))
  (while (LocalVariables|GetWorking)
    (LocalVariables|SetWorking false)
    (LocalVariables|SetConnectedTiles (LocalVariables|GetTiles)))
  (for _array_element (LocalVariables|GetConnectedTiles)
    (Utilities|Array|Add (LocalVariables|GetExtents_X) (.X (Utilities|Struct|BreakIntVector _array_element)))
    (Utilities|Array|Add (LocalVariables|GetExtents_Y) (.Z (Utilities|Struct|BreakIntVector _array_element))))
  (return (LocalVariables|GetConnectedTiles) (LocalVariables|GetRootLocation) (Utilities|Struct|MakeIntVector (.MaxValue (Math|Integer|MaxOfIntArray (LocalVariables|GetExtents_X))) 0 (.MaxValue (Math|Integer|MaxOfIntArray (LocalVariables|GetExtents_Y))))))

(fn SpawnMaps
  (for (_array_element _array_index) (Variables|Default|GetDungeonMaps)
    (Variables|StartingRoom|SetRoomCounter _array_index)
    (CallFunction|RandomRoom (.x (* (Math|Conversions|ToVector(Float) _array_element) (Variables|EditorTools|GetXScale))) (.y (* (Math|Conversions|ToVector(Float) _array_element) (Variables|EditorTools|GetZScale))) (.z (* (Math|Conversions|ToVector(Float) _array_element) (Variables|EditorTools|GetZScale))))))

(fn RandomRoom
  (params (X :type Float%20%28single-precision%29) (Y :type Float%20%28single-precision%29) (Z :type Float%20%28single-precision%29))
  (LocalVariables|SetXVal X)
  (LocalVariables|SetYVal Y)
  (LocalVariables|SetZVal Z)
  (if (< (Variables|StartingRoom|GetRoomCounter) 1)
    (Game|SpawnActorfromClass "/Game/Blueprints/Dungeon/Rooms/StartRoom/StartingRoom_BP.StartingRoom_BP_C" (Math|Transform|MakeTransform (Math|Vector|MakeVector (LocalVariables|GetXVal) (LocalVariables|GetYVal) (LocalVariables|GetZVal)) "0, 0, 0" "1,1,1") "Undefined" 0 0)
    (bind _returnvalue (Game|SpawnActorfromClass "/Game/Blueprints/Camera/RoomCamera_BP.RoomCamera_BP_C" (Math|Transform|MakeTransform (Math|Vector|MakeVector 0.0 0.0 0.0) "0, 0, 0" "1,1,1") "Undefined" 0 0))
    (bind _output_get (Variables|Default|SetInitialCam _returnvalue))
    (bind _asgame_instance (Utilities|Casting|CastToGame_Instance (Game|GetGameInstance)))
    (Default|SetCamera _asgame_instance _output_get)
    (else
      (Game|SpawnActorfromClass (Utilities|Select :Index (Variables|Default|GetRandomRoomPick) :NewEnumerator3 0 :NewEnumerator0 "/Game/Blueprints/Dungeon/Rooms/BP_Room_Easy1.BP_Room_Easy1_C" :NewEnumerator1 "/Game/Blueprints/Dungeon/Rooms/BP_Room_Easy1.BP_Room_Easy1_C" :NewEnumerator2 "/Game/Blueprints/Dungeon/Rooms/BP_Room_Easy1.BP_Room_Easy1_C" :NewEnumerator4 0 :NewEnumerator5 0 :NewEnumerator6 "/Game/Blueprints/Dungeon/Rooms/BP_Room_Easy1.BP_Room_Easy1_C" :NewEnumerator7 0 :NewEnumerator8 "/Game/Blueprints/Dungeon/Rooms/Treasure/BP_Room_Treasure.BP_Room_Treasure_C" :NewEnumerator9 "/Game/Blueprints/Dungeon/Rooms/Boss/BP_Room_Boss.BP_Room_Boss_C" :NewEnumerator11 0) (Math|Transform|MakeTransform (Math|Vector|MakeVector (LocalVariables|GetXVal) (LocalVariables|GetYVal) (LocalVariables|GetZVal)) "0, 0, 0" "1,1,1") "Undefined" 0 0)
      (Game|SpawnActorfromClass "/Game/Blueprints/Camera/RoomCamera_BP.RoomCamera_BP_C" (Math|Transform|MakeTransform (Math|Vector|MakeVector (LocalVariables|GetXVal) (LocalVariables|GetYVal) (LocalVariables|GetZVal)) "0, 0, 0" "1,1,1") "Undefined" 0 0)))
  (return (LocalVariables|GetXVal) (LocalVariables|GetYVal) (LocalVariables|GetZVal)))