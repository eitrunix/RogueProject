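; BP_Room_Easy1 is a dungeon room actor whose tile map is shown only while the player is inside.
; On BeginPlay it spawns a room camera at its root and, for the start room, registers it as the starting camera in the Game Instance.
; RoomBoxTrigger overlaps with the player set an inside flag, which Tick turns into tile map visibility.
; The construction script assigns the tile map; the spawning trigger handler is empty.
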(event OnComponentBeginOverlap(RoomBoxTrigger)
  (params (OverlappedComponent :type Primitive%20Component%20Object%20Reference) (OtherActor :type Actor%20Object%20Reference) (OtherComp :type Primitive%20Component%20Object%20Reference) (OtherBodyIndex :type Integer) (bFromSweep :type Boolean) (SweepResult :type Hit%20Result%20Structure%20%28by%20ref%29))
  (Utilities|Casting|CastToMasterPlayer_BP OtherActor)
  (Variables|Default|SetInsideRoom true))

(event OnComponentEndOverlap(RoomBoxTrigger)
  (params (OverlappedComponent :type Primitive%20Component%20Object%20Reference) (OtherActor :type Actor%20Object%20Reference) (OtherComp :type Primitive%20Component%20Object%20Reference) (OtherBodyIndex :type Integer))
  (Utilities|Casting|CastToMasterPlayer_BP OtherActor)
  (Variables|Default|SetInsideRoom false))

(event OnComponentBeginOverlap(SpawningTrigger)
  (params (OverlappedComponent :type Primitive%20Component%20Object%20Reference) (OtherActor :type Actor%20Object%20Reference) (OtherComp :type Primitive%20Component%20Object%20Reference) (OtherBodyIndex :type Integer) (bFromSweep :type Boolean) (SweepResult :type Hit%20Result%20Structure%20%28by%20ref%29)))

(event EventBeginPlay
  (bind _returnvalue (Game|SpawnActorfromClass "/Game/Blueprints/Camera/RoomCamera_BP.RoomCamera_BP_C" (Transformation|GetWorldTransform (Variables|Default|GetDefaultSceneRoot)) "Undefined" 0 0))
  (if (Variables|Default|GetIsStartRoom)
    (bind _asgame_instance (Utilities|Casting|CastToGame_Instance (Game|GetGameInstance)))
    (Variables|/Game/Blueprints/Instance/Game_Instance.Game_Instance_C|SetCameraStart _asgame_instance _returnvalue)
    (Variables|Default|SetInsideRoom true)))

(event Collision|EventActorBeginOverlap
  (params (OtherActor :type Actor%20Object%20Reference)))

(event EventTick
  (params (DeltaSeconds :type Float%20%28single-precision%29))
  (if (Variables|Default|GetInsideRoom)
    (Rendering|SetVisibility (Variables|Default|GetRoomMap) true true)
    (else
      (Rendering|SetVisibility (Variables|Default|GetRoomMap) false true))))

(fn ConstructionScript
  (Class|PaperTileMapComponent|SetTileMap (Variables|Default|GetRoomMap) (Variables|Default|GetRoom%20Tile%20Map)))