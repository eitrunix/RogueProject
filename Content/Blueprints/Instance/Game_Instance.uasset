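; Game instance that stores the player's character selection and shared run state.
; SetPlayer records the chosen character and pawn, then switches on the character (Vr Guy, Ninja Frog, Pink Man, Mask Dude) to set exclusive selection flags.
; ResetSetPlayer stores the passed values but clears all flags.
; Simple setters hold the run-start flag, max and current health, and camera start value.
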(fn SetPlayer
  (params (Player :type Player%20Controller%20Object%20Reference) (Pawn :type PlayerSelect%20Enum :default "NewEnumerator0"))
  (Variables|PlayerVars|SetcurrentPlayer Pawn)
  (Variables|PlayerVars|Setplayer Player)
  (switch Utilities|FlowControl|Switch|SwitchonPlayerSelect (Variables|PlayerVars|GetcurrentPlayer)
    (:NewEnumerator0
      (Variables|PlayerSelect|SetPlayer1Sel true)
      (Variables|PlayerSelect|SetPlayer2Sel false)
      (Variables|PlayerSelect|SetPlayer3Sel false)
      (Variables|PlayerSelect|SetPlayer4Sel false))
    (:NewEnumerator1
      (Variables|PlayerSelect|SetPlayer1Sel false)
      (Variables|PlayerSelect|SetPlayer2Sel true)
      (Variables|PlayerSelect|SetPlayer3Sel false)
      (Variables|PlayerSelect|SetPlayer4Sel false))
    (:NewEnumerator2
      (Variables|PlayerSelect|SetPlayer1Sel false)
      (Variables|PlayerSelect|SetPlayer2Sel false)
      (Variables|PlayerSelect|SetPlayer3Sel true)
      (Variables|PlayerSelect|SetPlayer4Sel false))
    (:NewEnumerator3
      (Variables|PlayerSelect|SetPlayer1Sel false)
      (Variables|PlayerSelect|SetPlayer2Sel false)
      (Variables|PlayerSelect|SetPlayer3Sel false)
      (Variables|PlayerSelect|SetPlayer4Sel true))))

(fn ResetSetPlayer
  (params (Player :type Player%20Controller%20Object%20Reference) (Pawn :type PlayerSelect%20Enum :default "NewEnumerator0"))
  (Variables|PlayerVars|SetcurrentPlayer Pawn)
  (Variables|PlayerVars|Setplayer Player)
  (Variables|PlayerSelect|SetPlayer1Sel false)
  (Variables|PlayerSelect|SetPlayer2Sel false)
  (Variables|PlayerSelect|SetPlayer3Sel false)
  (Variables|PlayerSelect|SetPlayer4Sel false))

(fn SetRunStart
  (Variables|Default|SetRunStart true))

(fn SetMaxHealth
  (params (MaxHealth :type Integer))
  (Variables|PlayerVars|SetMAXHealth MaxHealth))

(fn SetCurrentHealth
  (params (CurrentHealth :type Integer))
  (Variables|PlayerVars|SetcurrentHealth CurrentHealth))

(fn SetCamera
  (params (CameraStart :type Room%20Camera%20BP%20Object%20Reference))
  (Variables|Default|SetCameraStart CameraStart))