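; Master enemy character for a 2D flipbook game, with ranged attack, knockback and death.
; Tick fires timed projectiles while Ranging, otherwise picks idle or walk animation, and turns the controller to face X velocity.
; Damage lowers health, then either launches the enemy back or destroys it after a short delay.
; SetFlipBook maps animation states to flipbooks; leftover jump, movement, ranging-toggle and test-damage logic is disconnected.
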(event Custom|ToggleAttack
  ;[1 1 1] Basic Attack and Auto Attack
  (Variables|Combat|SetAttackIng false))

(event Custom|UpdateAnimation
  ;[1 1 1] Handle Animation
  (if (not (Variables|IsHit|GetisHit))
    (if (AI|Components|NavMovement|IsFalling (Variables|Character|GetCharacterMovement))
      (CallFunction|SetFlipBook "NewEnumerator0")
      (else
        (CallFunction|SetFlipBook (select (> (Math|Vector|VectorLength (Transformation|GetVelocity)) 0.0) "NewEnumerator2" "NewEnumerator0"))))))

(event Custom|AutoActtack
  (bind _attackposition (Variables|Default|GetAttackPosition))
  (bind _projsize (Variables|EnemyProjectileVar|GetProjSize))
  (bind _returnvalue (Transformation|GetWorldTransform _attackposition))
  (bind _returnvalue_2 (/ _projsize 1e+01))
  ;[1 1 1] Basic Attack and Auto Attack
  (if (not (Variables|Combat|GetAttackIng))
    (bind _returnvalue_3 (Game|SpawnActorfromClass (Variables|EnemyProjectileVar|GetProjectile) (Math|Transform|MakeTransform (.location _returnvalue) (.rotation _returnvalue) (Math|Vector|MakeVector _returnvalue_2 (.y (.scale _returnvalue)) _returnvalue_2)) "Undefined" 0 0))
    (Variables|Default|SetTmpBullet _returnvalue_3)
    (Utilities|Time|SetTimerbyEvent (delegate Custom|ToggleAttack) (Variables|EnemyProjectileVar|GetAttackSpeed))
    (Variables|Combat|SetAttackIng true)))

(event Game|Damage|EventAnyDamage
  (params (Damage :type Float%20%28single-precision%29) (DamageType :type Damage%20Type%20Object%20Reference) (InstigatedBy :type Controller%20Object%20Reference) (DamageCauser :type Actor%20Object%20Reference))
  ;[1 1 1] On Hit sstuff
  (CallFunction|SetFlipBook "NewEnumerator1")
  (bind _output_get (Variables|EnemyVars|Setcurrent_Health (- (Variables|EnemyVars|Getcurrent_Health) (Math|Float|Truncate Damage))))
  (if (< _output_get 1)
    (CallFunction|SetFlipBook "NewEnumerator7")
    (Utilities|FlowControl|Delay 0.5)
    (Actor|DestroyActor)
    (elif (Variables|Animation|GetbisMovingRight)
      (Character|LaunchCharacter (Math|Vector|MakeVector -1.1e+02 0.0 1e+02) true true)
      (else
        (Character|LaunchCharacter (Math|Vector|MakeVector 1.1e+02 0.0 1e+02) true true)))))

(event EventTick
  (params (DeltaSeconds :type Float%20%28single-precision%29))
  ;[1 1 1] Tick - Updates animation
  (if (Variables|Combat|GetRanging)
    (CallFunction|AutoActtack)
    (else
      (CallFunction|UpdateAnimation)))
  (Math|Float|CompareFloat (.X (Math|Vector|BreakVector (Variables|/Script/Engine.MovementComponent|GetVelocity (Pawn|GetMovementComponent)))) 0.0
    (:>
      (Pawn|SetControlRotation (Pawn|GetController) (Math|Rotator|MakeRotator 0.0 0.0 0.0) :!label _label))
    (:==
      (if (Variables|Animation|GetbisMovingRight)
        (goto _label)
        (else
          (Pawn|SetControlRotation (Pawn|GetController) (Math|Rotator|MakeRotator 0.0 0.0 1.8e+02) :!label _label_2))))
    (:<
      (goto _label_2))))

(event EventBeginPlay
  ;[1 1 1] Startup
  (Class|ActorComponent|SetIsReplicated (Variables|Default|GetSprite) true))

(event Input|ActionEvents|InputActionRangedAttack
  (params (Key :type Key%20Structure :default "None"))
  ;[1 1 1] Handle Animation
)

(event Input|ActionEvents|InputActionJump
  (params (Key :type Key%20Structure :default "None"))
  ;[1 1 1] Handle movement
)

(event Input|AxisEvents|InputAxisMoveRight
  (params (AxisValue :type Float%20%28single-precision%29))
  ;[1 1 1] Handle movement
)

(event Input|KeyboardEvents|J
  (params (Key :type Key%20Structure :default "None"))
  ;[1 1 1] TESTING DAMAGE REMOVE
)

(event Input|TouchEvents|InputTouch
  (params (Location :type Vector) (FingerIndex :type ETouchIndex%20Enum))
  ;[1 1 1] Handle movement
)

(fn ConstructionScript)

(fn SetFlipBook
  (params (NextState :type EnemyFlipBook%20Enum :default "NewEnumerator0"))
  (Variables|EnemyVars|SetFlipBookAnims NextState)
  (Sprite|SetFlipbook (Variables|Default|GetSprite) (Utilities|Select :Index (Variables|EnemyVars|GetFlipBookAnims) :NewEnumerator0 (Variables|Animation|Getfb_Idle) :NewEnumerator1 (Variables|Animation|Getfb_hit1) :NewEnumerator7 (Variables|Animation|Getfb_hit2) :NewEnumerator2 (Variables|Animation|Getfb_walk1) :NewEnumerator3 (Variables|Animation|Getfb_walk2) :NewEnumerator4 (Variables|Animation|Getfb_attack1) :NewEnumerator5 (Variables|Animation|Getfb_attack2) :NewEnumerator6 (Variables|Animation|Getfb_death)))
  (return))