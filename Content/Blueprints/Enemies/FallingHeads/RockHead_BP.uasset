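; RockHead_BP is a falling-head trap enemy that drops when the player enters its sight volume, then returns to its start position.
; Sight overlap plays a blink flipbook, enables gravity on Body, then after a delay a timeline lerps it back and re-arms it.
; Body overlap destroys basic attacks and damages other actors.
; HeadType picks a rock or spike idle flipbook, but animation states use only rock flipbooks.
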(event OnComponentBeginOverlap(Sight)
  (params (OverlappedComponent :type Primitive%20Component%20Object%20Reference) (OtherActor :type Actor%20Object%20Reference) (OtherComp :type Primitive%20Component%20Object%20Reference) (OtherBodyIndex :type Integer) (bFromSweep :type Boolean) (SweepResult :type Hit%20Result%20Structure%20%28by%20ref%29))
  (if (not (Variables|Default|GetMoved))
    (Utilities|Casting|CastToMasterPlayer_BP OtherActor)
    (CallFunction|SetFlipBook "NewEnumerator3")
    (Utilities|FlowControl|Delay 0.25)
    (Physics|SetEnableGravity (Variables|Default|GetBody) true)
    (Variables|Default|SetMoved true)
    (Utilities|FlowControl|Delay 2.0)
    (Variables|Default|SetfallenPosition (Transformation|GetActorLocation))
    (CallFunction|SetFlipBook "NewEnumerator3")
    (Physics|SetEnableGravity (Variables|Default|GetBody) false)
    (CallFunction|SetFlipBook "NewEnumerator1")
    (bind _newtrack_1 (Timeline|FallREset PlayFromStart)
      (:Update
        (Transformation|SetRelativeLocation (Variables|Default|GetBody) (Math|Vector|Lerp(Vector) (Variables|Default|GetfallenPosition) (Variables|Default|GetInitialPosition) _newtrack_1) false false))
      (:Finished
        (Variables|Default|SetMoved false)))))

(event OnComponentBeginOverlap(Body)
  (params (OverlappedComponent :type Primitive%20Component%20Object%20Reference) (OtherActor :type Actor%20Object%20Reference) (OtherComp :type Primitive%20Component%20Object%20Reference) (OtherBodyIndex :type Integer) (bFromSweep :type Boolean) (SweepResult :type Hit%20Result%20Structure%20%28by%20ref%29))
  (Utilities|Casting|CastToBasicAttack_BP OtherActor
    (:then
      (Actor|DestroyActor OtherActor))
    (:CastFailed
      (Game|Damage|ApplyDamage OtherActor (Variables|Default|GetDamage) 0 0))))

(event EventBeginPlay
  (Variables|Default|SetInitialPosition (Transformation|GetActorLocation)))

(event Collision|EventActorBeginOverlap
  (params (OtherActor :type Actor%20Object%20Reference)))

(event EventTick
  (params (DeltaSeconds :type Float%20%28single-precision%29)))

(fn ConstructionScript)

(fn SetHeadType
  (params (NewParam :type FallingHeadType%20Enum :default "NewEnumerator0"))
  (bind _output_get (Variables|Default|SetheadType NewParam))
  (Sprite|SetFlipbook (Variables|Default|GetPaperFlipbook) (Utilities|Select :Index _output_get :NewEnumerator0 "/Game/Art_Textures/Traps/Rock_Head/Anims/Idle_RockHead.Idle_RockHead" :NewEnumerator1 "/Game/Art_Textures/Traps/Spike_Head/Anims/Idle_SpikeHead.Idle_SpikeHead")))

(fn SetFlipBook
  (params (NewParam :type TrapAnims%20Enum :default "NewEnumerator1"))
  (Variables|Default|SetCurrentAnimState NewParam)
  (Sprite|SetFlipbook (Variables|Default|GetPaperFlipbook) (Utilities|Select :Index (Variables|Default|GetCurrentAnimState) :NewEnumerator1 "/Game/Art_Textures/Traps/Rock_Head/Anims/Idle_RockHead.Idle_RockHead" :NewEnumerator3 "/Game/Art_Textures/Traps/Rock_Head/Anims/Blink__42x42_RockHead.Blink__42x42_RockHead" :NewEnumerator4 0 :NewEnumerator5 "/Game/Art_Textures/Traps/Rock_Head/Anims/Bottom_Hit__42x42__RockHead.Bottom_Hit__42x42__RockHead" :NewEnumerator6 0))
  (return))