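; Spike Head enemy from the FallingHeads set, a Paper2D actor that supplies the head's flipbook animations.
; SetFlipBook stores the requested animation state and selects the matching idle, blink or bottom-hit flipbook, leaving the Off and Misc2 states unassigned.
; The event graph holds only disabled stubs and the construction script just calls the parent, so this Blueprint defines no movement or damage logic itself.
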(event EventBeginPlay
  (|CallParentFunction) ; This node is disabled and will not be called.\nDrag off pins to build functionality.
)

(event Collision|EventActorBeginOverlap
  (params (OtherActor :type Actor%20Object%20Reference))
  (|CallParentFunction OtherActor) ; This node is disabled and will not be called.\nDrag off pins to build functionality.
)

(event EventTick
  (params (DeltaSeconds :type Float%20%28single-precision%29))
  (|CallParentFunction DeltaSeconds) ; This node is disabled and will not be called.\nDrag off pins to build functionality.
)

(fn ConstructionScript
  (|CallParentFunction))

(fn SetFlipBook
  (params (NewParam :type TrapAnims%20Enum :default "NewEnumerator1"))
  (Variables|Default|SetCurrentAnimState NewParam)
  (Sprite|SetFlipbook (Variables|Default|GetPaperFlipbook) (Utilities|Select :Index (Variables|Default|GetCurrentAnimState) :NewEnumerator1 "/Game/Art_Textures/Traps/Spike_Head/Anims/Idle_SpikeHead.Idle_SpikeHead" :NewEnumerator3 "/Game/Art_Textures/Traps/Spike_Head/Anims/Blink__54x52__SpikeHead.Blink__54x52__SpikeHead" :NewEnumerator4 0 :NewEnumerator5 "/Game/Art_Textures/Traps/Spike_Head/Anims/Bottom_Hit__54x52__SpikeHead.Bottom_Hit__54x52__SpikeHead" :NewEnumerator6 0))
  (return))