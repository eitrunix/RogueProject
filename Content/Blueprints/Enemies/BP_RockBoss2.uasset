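; BP_RockBoss2 is a rock boss stage that splits into four BP_RockBoss3 actors when destroyed.
; The Destroyed event runs four identical spawns through a sequence, copying its rotation, scale and X/Z location while leaving Y unwired.
; All four spawn at the same point with AlwaysSpawn, so collision does not block them.
; The graph holds no other active logic.
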(event EventBeginPlay
  (|CallParentFunction) ; This node is disabled and will not be called.\nDrag off pins to build functionality.
)

(event Collision|EventActorBeginOverlap
  (params (OtherActor :type Actor%20Object%20Reference)))

(event EventTick
  (params (DeltaSeconds :type Float%20%28single-precision%29))
  (|CallParentFunction DeltaSeconds) ; This node is disabled and will not be called.\nDrag off pins to build functionality.
)

(event EventDestroyed
  (bind _returnvalue (Transformation|GetActorTransform))
  (Utilities|FlowControl|Sequence
    (:then_0
      (Game|SpawnActorfromClass "/Game/Blueprints/Enemies/BP_RockBoss3.BP_RockBoss3_C" (Math|Transform|MakeTransform (Math|Vector|MakeVector (.x (.location _returnvalue)) 0.0 (.z (.location _returnvalue))) (.rotation _returnvalue) (.scale _returnvalue)) "AlwaysSpawn" 0 0))
    (:then_1
      (Game|SpawnActorfromClass "/Game/Blueprints/Enemies/BP_RockBoss3.BP_RockBoss3_C" (Math|Transform|MakeTransform (Math|Vector|MakeVector (.x (.location _returnvalue)) 0.0 (.z (.location _returnvalue))) (.rotation _returnvalue) (.scale _returnvalue)) "AlwaysSpawn" 0 0))
    (:then_2
      (Game|SpawnActorfromClass "/Game/Blueprints/Enemies/BP_RockBoss3.BP_RockBoss3_C" (Math|Transform|MakeTransform (Math|Vector|MakeVector (.x (.location _returnvalue)) 0.0 (.z (.location _returnvalue))) (.rotation _returnvalue) (.scale _returnvalue)) "AlwaysSpawn" 0 0))
    (:then_3
      (Game|SpawnActorfromClass "/Game/Blueprints/Enemies/BP_RockBoss3.BP_RockBoss3_C" (Math|Transform|MakeTransform (Math|Vector|MakeVector (.x (.location _returnvalue)) 0.0 (.z (.location _returnvalue))) (.rotation _returnvalue) (.scale _returnvalue)) "AlwaysSpawn" 0 0))))

(fn ConstructionScript
  (|CallParentFunction))