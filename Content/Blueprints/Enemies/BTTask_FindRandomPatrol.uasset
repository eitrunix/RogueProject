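; Behavior tree task that picks a random patrol destination for enemies derived from Master_Enemy_BP.
; It sets the enemy's walk speed to the patrol speed, then looks for a random reachable point within the patrol radius around the pawn.
; The result is written to the PatrolLocation blackboard key, falling back to the pawn's current location if no point is found.
; The task fails only when the pawn cast fails.
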(event EventReceiveExecuteAI
  (params (OwnerController :type AI%20Controller%20Object%20Reference) (ControlledPawn :type Pawn%20Object%20Reference))
  (bind _returnvalue (Transformation|GetActorLocation ControlledPawn))
  (bind _patrolradius (Variables|Default|GetPatrolRadius))
  (bind (_randomlocation _returnvalue_2) (AI|Navigation|GetRandomReachablePointinRadius _returnvalue _patrolradius 0 0))
  (bind _asmaster_enemy_bp (Utilities|Casting|CastToMaster_Enemy_BP ControlledPawn)
    (:then
      (Default|UpdateWalkSpeed _asmaster_enemy_bp (Variables|Default|GetPatrol%20Speed))
      (if _returnvalue_2
        (AI|BehaviorTree|SetBlackboardValueasVector (Variables|Default|GetPatrolLocation) _randomlocation)
        (else
          (AI|BehaviorTree|SetBlackboardValueasVector (Variables|Default|GetPatrolLocation) _returnvalue)))
      (AI|BehaviorTree|FinishExecute true))
    (:CastFailed
      (AI|BehaviorTree|FinishExecute false))))