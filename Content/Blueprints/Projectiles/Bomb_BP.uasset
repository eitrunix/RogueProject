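; Timed bomb projectile that switches to an explosion flipbook and damages non-player actors.
; A timer set on BeginPlay calls Explode, which stops projectile movement, sets the Exploded flag and destroys the actor after a delay.
; ExplosionRadius overlaps that begin while Exploded is set exempt MasterPlayer_BP and call ApplyDamage for anything else, so actors already inside at detonation are not checked.
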(event OnComponentBeginOverlap(ExplosionRadius)
  (params (OverlappedComponent :type Primitive%20Component%20Object%20Reference) (OtherActor :type Actor%20Object%20Reference) (OtherComp :type Primitive%20Component%20Object%20Reference) (OtherBodyIndex :type Integer) (bFromSweep :type Boolean) (SweepResult :type Hit%20Result%20Structure%20%28by%20ref%29))
  (if (Variables|Default|GetExploded)
    (Utilities|Casting|CastToMasterPlayer_BP OtherActor
      (:then
        (Development|PrintString "Playe rCant bomb self"))
      (:CastFailed
        (Game|Damage|ApplyDamage 0 3.0 0 0)
        (Development|PrintString "Monster took damage")))))

(event Custom|Explode
  (Sprite|SetFlipbook (Variables|Default|GetBomb) "/Game/Projectiles/1-BOMB/3-Explotion/Bomb_Explode.Bomb_Explode")
  (Variables|/Script/Engine.ProjectileMovementComponent|SetbSimulationEnabled (Variables|Default|GetProjectileMovement) false)
  (Variables|Default|SetExploded true)
  (Utilities|FlowControl|Delay (Variables|Default|GetDestroyAfterXSec))
  (Actor|DestroyActor))

(event EventBeginPlay
  (Utilities|Time|SetTimerbyEvent (delegate Custom|Explode) (Variables|Default|GetTimeToDetonate)))

(event Collision|EventActorBeginOverlap
  (params (OtherActor :type Actor%20Object%20Reference)))

(event EventTick
  (params (DeltaSeconds :type Float%20%28single-precision%29)))

(fn ConstructionScript)