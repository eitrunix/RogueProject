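; BasicAttack_BP is the player's short-lived basic attack projectile, drawn with a Paper2D flipbook chosen by the selected character in Game_Instance.
; On spawn it scales itself from the player's ProjSize and starts a timer that destroys it.
; Its sphere overlap applies BulletDamage to enemies or zeroes a trap collider's velocity, then destroys the projectile.
; SetBulletDamage exposes the damage value for setting.
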(event OnComponentBeginOverlap(Sphere)
  (params (OverlappedComponent :type Primitive%20Component%20Object%20Reference) (OtherActor :type Actor%20Object%20Reference) (OtherComp :type Primitive%20Component%20Object%20Reference) (OtherBodyIndex :type Integer) (bFromSweep :type Boolean) (SweepResult :type Hit%20Result%20Structure%20%28by%20ref%29))
  (bind _asmaster_enemy_bp (Utilities|Casting|CastToMaster_Enemy_BP OtherActor)
    (:then
      (Development|PrintString "Hit Enemy")
      (Game|Damage|ApplyDamage _asmaster_enemy_bp (Variables|Default|GetBulletDamage) 0 0)
      (Actor|DestroyActor :!label _label))
    (:CastFailed
      (bind _astrap_master_bp (Utilities|Casting|CastToTrapMaster_BP OtherActor)
        (:then
          (Physics|SetPhysicsLinearVelocity (Variables|/Game/Blueprints/Traps/TrapMaster_BP.TrapMaster_BP_C|GetUnitCollider _astrap_master_bp) "0, 0, 0" false "None")
          (goto _label))
        (:CastFailed
          (Utilities|Casting|CastToMasterPlayer_BP OtherActor))))))

(event Custom|BulletLife
  (Actor|DestroyActor))

(event EventBeginPlay
  (Utilities|Time|SetTimerbyEvent (delegate Custom|BulletLife) 0.75)
  (bind _asmaster_player_bp (Utilities|Casting|CastToMasterPlayer_BP (Game|GetPlayerCharacter 0)))
  (Transformation|SetActorRelativeScale3D (Math|Vector|MakeVector (/ (Variables|/Game/Blueprints/Player/MasterPlayer_BP.MasterPlayer_BP_C|GetProjSize _asmaster_player_bp) 1e+01) (/ (Variables|/Game/Blueprints/Player/MasterPlayer_BP.MasterPlayer_BP_C|GetProjSize _asmaster_player_bp) 1e+01) (/ (Variables|/Game/Blueprints/Player/MasterPlayer_BP.MasterPlayer_BP_C|GetProjSize _asmaster_player_bp) 1e+01))))

(event Collision|EventActorBeginOverlap
  (params (OtherActor :type Actor%20Object%20Reference)))

(event EventTick
  (params (DeltaSeconds :type Float%20%28single-precision%29)))

(fn ConstructionScript
  (bind _asgame_instance (Utilities|Casting|CastToGame_Instance (Game|GetGameInstance)))
  (Sprite|SetFlipbook (Variables|Default|GetPaperFlipbook) (Utilities|Select :Index (Variables|/Game/Blueprints/Instance/Game_Instance.Game_Instance_C|GetcurrentPlayer _asgame_instance) :NewEnumerator0 "/Game/Art_Textures/Projectiles/NormalAttack/VRGuy_Proj_Flipbook.VRGuy_Proj_Flipbook" :NewEnumerator1 "/Game/Art_Textures/Projectiles/NormalAttack/NinjaFrog_Proj_Flipbook.NinjaFrog_Proj_Flipbook" :NewEnumerator2 "/Game/Art_Textures/Projectiles/NormalAttack/PinkDude_Proj_Flipbook.PinkDude_Proj_Flipbook" :NewEnumerator3 "/Game/Art_Textures/Projectiles/NormalAttack/MaskMan_Proj_Flipbook.MaskMan_Proj_Flipbook" :NewEnumerator4 0)))

(fn SetBulletDamage
  (params (BulletDamage :type Float%20%28single-precision%29))
  (Variables|Default|SetBulletDamage BulletDamage))