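; Base trap actor for a 2D Paper2D game, selecting its flipbook sprite from a Trap type enum covering fire, fan, trampoline, heads, saw, spikes and falling platform.
; The construction script previews the type's idle or off flipbook on the Sprite.
; On BeginPlay, the IsOn flag switches the Sprite between the OnAnimation and OffAnimation flipbooks.
; No trap gameplay logic, overlap or tick behavior is implemented in this graph.
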(event EventBeginPlay
  (if (Variables|Default|GetIsOn)
    (Sprite|SetFlipbook (Variables|Default|GetSprite) (Variables|Default|GetOnAnimation))
    (else
      (Sprite|SetFlipbook (Variables|Default|GetSprite) (Variables|Default|GetOffAnimation)))))

(event Collision|EventActorBeginOverlap
  (params (OtherActor :type Actor%20Object%20Reference)))

(event EventTick
  (params (DeltaSeconds :type Float%20%28single-precision%29)))

(fn ConstructionScript
  (Sprite|SetFlipbook (Variables|Default|GetSprite) (Utilities|Select :Index (Variables|Default|GetTrap) :NewEnumerator0 "/Game/Art_Textures/Traps/Fire/Anims/Off_FireTrap.Off_FireTrap" :NewEnumerator1 "/Game/Art_Textures/Traps/Fan/Anims/Fan_Off.Fan_Off" :NewEnumerator2 "/Game/Art_Textures/Traps/Trampoline/Anims/Idle_Spring.Idle_Spring" :NewEnumerator3 "/Game/Art_Textures/Traps/Rock_Head/Anims/Idle_RockHead.Idle_RockHead" :NewEnumerator4 "/Game/Art_Textures/Traps/Spike_Head/Anims/Idle_SpikeHead.Idle_SpikeHead" :NewEnumerator5 "/Game/Art_Textures/Traps/Saw/Anims/Off_Saw.Off_Saw" :NewEnumerator6 "/Game/Art_Textures/Traps/Spikes/Idle_Flipbook_Spikes.Idle_Flipbook_Spikes" :NewEnumerator7 "/Game/Art_Textures/Traps/Falling_Platforms/Anims/Platform_On__32x10.Platform_On__32x10")))