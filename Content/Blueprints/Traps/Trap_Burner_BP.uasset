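; A fire burner trap with flipbook visuals that damages the player or enemies beginning overlap with its hit collider while it is on.
; Tick uses latent Delays to alternate timed on and off phases, showing a ReadyFire warning animation before ignition.
; The collider drops on BeginPlay and switch-off, but the node that would raise it is unconnected.
; The construction script sets the inherited trap type and fire animations.
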(event OnComponentBeginOverlap(HitColliter)
  (params (OverlappedComponent :type Primitive%20Component%20Object%20Reference) (OtherActor :type Actor%20Object%20Reference) (OtherComp :type Primitive%20Component%20Object%20Reference) (OtherBodyIndex :type Integer) (bFromSweep :type Boolean) (SweepResult :type Hit%20Result%20Structure%20%28by%20ref%29))
  (bind _damage (Variables|Default|GetDamage))
  (if (Variables|Default|GetIsOn)
    (bind _asmaster_player_bp (Utilities|Casting|CastToMasterPlayer_BP OtherActor)
      (:then
        (Game|Damage|ApplyDamage _asmaster_player_bp _damage 0 0))
      (:CastFailed
        (bind _asbkup_master_enemy (Utilities|Casting|CastToBKUP_MasterEnemy OtherActor))
        (Game|Damage|ApplyDamage _asbkup_master_enemy _damage 0 0)))))

(event EventBeginPlay
  (|CallParentFunction)
  (Transformation|SetRelativeLocation (Variables|Default|GetHitColliter) "0, 0,-10.000000" false false))

(event Collision|EventActorBeginOverlap
  (params (OtherActor :type Actor%20Object%20Reference))
  (|CallParentFunction OtherActor) ; This node is disabled and will not be called.\nDrag off pins to build functionality.
)

(event EventTick
  (params (DeltaSeconds :type Float%20%28single-precision%29))
  (bind _sprite (Variables|Default|GetSprite))
  (|CallParentFunction DeltaSeconds)
  (if (Variables|Default|GetIsOn)
    (Utilities|FlowControl|Delay (Variables|Default|GetTimeOn))
    (Variables|Default|SetIsOn false)
    (Sprite|SetFlipbook _sprite (Variables|Default|GetOffAnimation))
    (Transformation|SetRelativeLocation (Variables|Default|GetHitColliter) "0, 0,-10.000000" false false)
    (else
      (Utilities|FlowControl|Delay (- (Variables|Default|GetTimeOff) (Variables|Default|Getflickerlight)))
      (Sprite|SetFlipbook (Variables|Default|GetSprite) "/Game/Art_Textures/Traps/Fire/Anims/ReadyFire.ReadyFire")
      (Utilities|FlowControl|Delay (- (Variables|Default|GetTimeOff) (Variables|Default|Getflickerlight)))
      (Variables|Default|SetIsOn true)
      (Sprite|SetFlipbook _sprite (Variables|Default|GetOnAnimation)))))

(fn ConstructionScript
  (|CallParentFunction)
  (Variables|Default|SetTrap "NewEnumerator0")
  (Variables|Default|SetOnAnimation "/Game/Art_Textures/Traps/Fire/Anims/On__16x32__FireTrap.On__16x32__FireTrap")
  (Variables|Default|SetOffAnimation "/Game/Art_Textures/Traps/Fire/Anims/Off_FireTrap.Off_FireTrap"))