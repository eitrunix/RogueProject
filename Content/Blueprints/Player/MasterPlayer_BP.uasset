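; Base 2D side-scrolling player character with movement, jumping, timed projectile auto-fire, item use and damage handling.
; Tick fires or uses items from held-input flags, picks flipbooks through a state selector and turns the controller to face travel direction.
; Damage triggers timed invulnerability and knockback, or death and a Stage1 reload.
; While Game_Instance.RunStart is set, every tick creates a GameHud and copies health to the Game Instance.
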(event Custom|InvulnFrames
  ;[1 1 1] On Hit sstuff
  (Variables|PlayerHit|SetInvuln true)
  (Utilities|Time|SetTimerbyEvent (delegate Custom|Disable) 0.74))

(event Custom|Disable
  ;[1 1 1] On Hit sstuff
  (Variables|PlayerHit|SetInvuln false))

(event Custom|ToggleAttack
  ;[1 1 1] Handle Animation
  ;;[1 1 1] Basic Attack and Auto Attack
  (Variables|Combat|SetAttackIng false))

(event Custom|UpdateAnimation
  ;[1 1 1] Handle Animation
  (if (not (Variables|PlayerHit|GetisHit))
    (if (AI|Components|NavMovement|IsFalling (Variables|Character|GetCharacterMovement))
      (CallFunction|SetFlipBook "NewEnumerator7")
      (else
        (CallFunction|SetFlipBook (select (> (Math|Vector|VectorLength (Transformation|GetVelocity)) 0.0) "NewEnumerator4" "NewEnumerator0"))))))

(event Custom|DisableHit
  ;[1 1 1] On Hit sstuff
  (Variables|PlayerHit|SetisHit false))

(event Custom|SetRunStartedEvent
  ;[1 1 1] Tick - Updates animation
  (bind _asgame_instance (Utilities|Casting|CastToGame_Instance (Game|GetGameInstance)))
  (if (Variables|/Game/Blueprints/Instance/Game_Instance.Game_Instance_C|GetRunStart _asgame_instance)
    (CallFunction|SetRunStarted)))

(event Custom|AutoActtack
  (bind _attackposition (Variables|Default|GetAttackPosition))
  (bind _projsize (Variables|PlayerProjectileVar|GetProjSize))
  (bind _returnvalue (Transformation|GetWorldTransform _attackposition))
  (bind _returnvalue_2 (/ _projsize 1e+01))
  ;[1 1 1] Basic Attack and Auto Attack
  (if (not (Variables|Combat|GetAttackIng))
    ;[1 1 1] Handle Animation
    (bind _returnvalue_3 (Game|SpawnActorfromClass (Variables|PlayerProjectileVar|GetProjectile) (Math|Transform|MakeTransform (.location _returnvalue) (.rotation _returnvalue) (Math|Vector|MakeVector _returnvalue_2 (.y (.scale _returnvalue)) _returnvalue_2)) "Undefined" 0 0))
    (bind _output_get (Variables|Default|SetTmpBullet _returnvalue_3))
    (bind _asbasic_attack_bp (Utilities|Casting|CastToBasicAttack_BP _output_get))
    (Default|SetBulletDamage _asbasic_attack_bp (Variables|PlayerProjectileVar|GetBulletDamage))
    (Utilities|Time|SetTimerbyEvent (delegate Custom|ToggleAttack) (Variables|PlayerProjectileVar|GetAttackSpeed))
    (Variables|Combat|SetAttackIng true)))

(event Custom|ItemCD
  ;[1 1 1] Handle Animation
  ;;[1 1 1] UseItem
  (Variables|Items|SetIsOffCD false))

(event Custom|UseItem
  ;[1 1 1] Handle Animation
  ;;[1 1 1] UseItem
  (if (not (Variables|Items|GetIsOffCD))
    (Game|SpawnActorfromClass (Variables|Items|GetItem) (Transformation|GetWorldTransform (Variables|Default|GetAttackPosition)) "Undefined" 0 0)
    (Utilities|Time|SetTimerbyEvent (delegate Custom|ItemCD) (Variables|Items|GetItemUseCD))
    (Variables|Items|SetIsOffCD true)))

(event Game|Damage|EventAnyDamage
  (params (Damage :type Float%20%28single-precision%29) (DamageType :type Damage%20Type%20Object%20Reference) (InstigatedBy :type Controller%20Object%20Reference) (DamageCauser :type Actor%20Object%20Reference))
  ;[1 1 1] On Hit sstuff
  (if (not (Variables|PlayerHit|GetInvuln))
    (CallFunction|InvulnFrames)
    (Variables|PlayerHit|SetisHit true)
    (CallFunction|SetFlipBook "NewEnumerator5")
    (bind _output_get (Variables|PlayerVars|Setcurrent_Health (- (Variables|PlayerVars|Getcurrent_Health) (Math|Float|Truncate Damage))))
    (if (< _output_get 1)
      (CallFunction|SetFlipBook "NewEnumerator8")
      (Input|DisableInput 0)
      (Utilities|FlowControl|Delay 0.75)
      (CallFunction|SetFlipBook "NewEnumerator10")
      (Development|PrintString "Reset Level, Add Input Confirm")
      (Utilities|FlowControl|Delay 0.75)
      (Game|OpenLevel(byName) "Stage1")
      (else
        (if (Variables|Animation|GetbisMovingRight)
          (Character|LaunchCharacter (Math|Vector|MakeVector -1.1e+02 0.0 1e+02) true true)
          (else
            (Character|LaunchCharacter (Math|Vector|MakeVector 1.1e+02 0.0 1e+02) true true)))
        (Utilities|Time|SetTimerbyEvent (delegate Custom|DisableHit) 0.74)))))

(event EventTick
  (params (DeltaSeconds :type Float%20%28single-precision%29))
  ;[1 1 1] Tick - Updates animation
  (CallFunction|SetRunStartedEvent)
  (if (Variables|Combat|GetRanging)
    (CallFunction|AutoActtack)
    (else
      (if (Variables|Items|GetUsingItem)
        (CallFunction|UseItem))
      (CallFunction|UpdateAnimation)))
  (Math|Float|CompareFloat (.X (Math|Vector|BreakVector (Variables|/Script/Engine.MovementComponent|GetVelocity (Pawn|GetMovementComponent)))) 0.0
    (:>
      (Pawn|SetControlRotation (Pawn|GetController) (Math|Rotator|MakeRotator 0.0 0.0 0.0) :!label _label))
    (:==
      (if (Variables|Animation|GetbisMovingRight)
        (goto _label)
        (else
          (Pawn|SetControlRotation (Pawn|GetController) (Math|Rotator|MakeRotator 0.0 0.0 1.8e+02) :!label _label_2))))
    (:<
      (goto _label_2))))

(event EventBeginPlay
  ;[1 1 1] Startup
  (Class|ActorComponent|SetIsReplicated (Variables|Default|GetSprite) true))

(event Input|ActionEvents|InputActionUseItem
  (params (Key :type Key%20Structure :default "None"))
  ;[1 1 1] Handle Animation
  (:Pressed
    (Variables|Items|SetUsingItem true))
  (:Released
    (Variables|Items|SetUsingItem false)))

(event Input|ActionEvents|InputActionRangedAttack
  (params (Key :type Key%20Structure :default "None"))
  ;[1 1 1] Handle Animation
  (:Pressed
    (Variables|Combat|SetRanging true))
  (:Released
    (Variables|Combat|SetRanging false)))

(event Input|ActionEvents|InputActionJump
  (params (Key :type Key%20Structure :default "None"))
  ;[1 1 1] Handle movement
  (:Pressed
    (Character|Jump)
    (if (Character|CanJump)
      (CallFunction|SetFlipBook "NewEnumerator3")
      (Utilities|FlowControl|Delay 0.1)
      (if (AI|Components|NavMovement|IsFalling (Variables|Character|GetCharacterMovement))
        (CallFunction|SetFlipBook "NewEnumerator7"))))
  (:Released
    (Character|StopJumping)))

(event Input|AxisEvents|InputAxisMoveRight
  (params (AxisValue :type Float%20%28single-precision%29))
  ;[1 1 1] Handle movement
  (if (> AxisValue 0.0)
    (Variables|Animation|SetbisMovingRight true)
    (elif (< AxisValue 0.0)
      (Variables|Animation|SetbisMovingRight false)))
  (Pawn|Input|AddMovementInput "1.000000, 0, 0" AxisValue false))

(event Input|TouchEvents|InputTouch
  (params (Location :type Vector) (FingerIndex :type ETouchIndex%20Enum))
  ;[1 1 1] Handle movement
  (:Released
    (Character|StopJumping)))

(fn ConstructionScript)

(fn SetFlipBook
  (params (NextState :type AnimState%20Enum :default "NewEnumerator0"))
  (Variables|PlayerVars|SetcurrentState NextState)
  (Sprite|SetFlipbook (Variables|Default|GetSprite) (Utilities|Select :Index (Variables|PlayerVars|GetcurrentState) :NewEnumerator0 (Variables|Animation|Getfb_Idle) :NewEnumerator1 (Variables|Animation|Getfb_dblJump) :NewEnumerator2 (Variables|Animation|Getfb_wallJump) :NewEnumerator3 (Variables|Animation|Getfb_jump) :NewEnumerator4 (Variables|Animation|Getfb_run) :NewEnumerator5 (Variables|Animation|Getfb_hit) :NewEnumerator7 (Variables|Animation|Getfb_fall) :NewEnumerator8 (Variables|Animation|Getfb_disappear) :NewEnumerator9 (Variables|Animation|Getfb_appear) :NewEnumerator10 0))
  (return))

(fn SetRunStarted
  (Variables|PlayerVars|SetRunStarted true)
  (bind _returnvalue (UserInterface|CreateWidget "/Game/Widgets/Hud/GameHud.GameHud_C"))
  (UserInterface|Viewport|AddtoViewport _returnvalue 0)
  (bind _asgame_instance (Utilities|Casting|CastToGame_Instance (Game|GetGameInstance)))
  (Default|SetMaxHealth _asgame_instance (Variables|PlayerVars|GetMAX_Health))
  (Default|SetCurrentHealth _asgame_instance (Variables|PlayerVars|Getcurrent_Health))
  (return))